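; BP_NPC is an NPC that shows voiced dialogue when the third-person character enters its sphere.
; On overlap it registers itself on the player, adds its W_Talk widget to the viewport and calls NextLine.
; Each NextLine steps through DT_NPCDialogue rows, setting text, playing voice and passing the speaker to the widget, which it removes after the last row.
; Leaving hides the widget and resets progress only if lines remain.
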(event `self.ReceiveBeginPlay`
  (bind _returnvalue (`|CreateWidget` "/Game/Widget/W_Talk.W_Talk_C"))
  (set `self.W_Talk` _returnvalue))

(event `self.Sphere.OnComponentBeginOverlap`
  (params (OverlappedComponent :type "PrimitiveComponent Object Reference") (OtherActor :type "Actor Object Reference") (OtherComp :type "PrimitiveComponent Object Reference") (OtherBodyIndex :type Integer) (bFromSweep :type Boolean) (SweepResult :type "HitResult Structure (by ref)"))
  (bind _asbp_third_person_character (cast `/Game/ThirdPerson/Blueprints/BP_ThirdPersonCharacter` OtherActor))
  (set `/Game/ThirdPerson/Blueprints/BP_ThirdPersonCharacter.NPC` self _asbp_third_person_character)
  (set `self.Player` _asbp_third_person_character)
  (`KismetSystemLibrary.PrintText` "Hello")
  (`UserWidget.AddToViewport` (`self.W_Talk`) 0)
  (`self.NextLine`))

(event `NextLine`
  (bind _lineindex (`self.LineIndex`))
  (bind _outrownames (`DataTableFunctionLibrary.GetDataTableRowNames` "/Game/Blueprints/DT_NPCDialogue.DT_NPCDialogue"))
  (if (< _lineindex (`KismetArrayLibrary.Array_Length` _outrownames))
    (bind _returnvalue (`|GetDataTableRow` "/Game/Blueprints/DT_NPCDialogue.DT_NPCDialogue" (`|GetArrayItem` _outrownames _lineindex))
      (:`then`
        (bind (_dialogue _voiceddialogue _speaker) (break `/Game/Blueprints/ST_NPCDialogue` _returnvalue))
        (set `TextBlock.Text` _dialogue (`/Game/Widget/W_Talk.TextBlock_67` (`self.W_Talk`)))
        (`GameplayStatics.PlaySound2D` _voiceddialogue 1.0 1.0 0.0 null null)
        (`/Game/Widget/W_Talk.AdvanceDialogue` (`self.W_Talk`) _speaker)
        (`/Engine/EditorBlueprintResources/StandardMacros.IncrementInt` (`self.LineIndex`))))
    (else
      (`Widget.RemoveFromParent` (`self.W_Talk`)))))

(event `self.Sphere.OnComponentEndOverlap`
  (params (OverlappedComponent :type "PrimitiveComponent Object Reference") (OtherActor :type "Actor Object Reference") (OtherComp :type "PrimitiveComponent Object Reference") (OtherBodyIndex :type Integer))
  (bind _w_talk (`self.W_Talk`))
  (cast `/Game/ThirdPerson/Blueprints/BP_ThirdPersonCharacter` OtherActor)
  (bind _outrownames (`DataTableFunctionLibrary.GetDataTableRowNames` "/Game/Blueprints/DT_NPCDialogue.DT_NPCDialogue"))
  (if (< (`self.LineIndex`) (`KismetArrayLibrary.Array_Length` _outrownames))
    (`Widget.RemoveFromParent` _w_talk)
    (set `self.LineIndex` 0)
    (else
      (`Widget.RemoveFromParent` _w_talk))))

(fn `UserConstructionScript`)